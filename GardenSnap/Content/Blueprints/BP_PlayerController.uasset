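; BP_PlayerController is a player controller that sets up the local player's view and HUD and handles score increases.
; On BeginPlay, for the local controller only, it blends the view to the level's CameraActor and adds a MainLayout widget to the viewport.
; Its IncreaseScore event adds a given amount to CurrentScore on the player's BP_PlayerState.
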(event `self.ReceiveBeginPlay`
  (if (`self.IsLocalPlayerController`)
    (bind _returnvalue (`GameplayStatics.GetActorOfClass` "/Script/Engine.CameraActor"))
    (`self.SetViewTargetWithBlend` _returnvalue)
    (bind _returnvalue_2 (`|GenericCreateObject` "/Game/Blueprints/MainLayout.MainLayout_C"))
    (`UserWidget.AddToViewport` _returnvalue_2 0)))

(event `IncreaseScore`
  (params (IncreaseAmount :type Integer))
  (bind _asbp_player_state (cast `/Game/Blueprints/BP_PlayerState` (`self.PlayerState`)))
  (set `/Game/Blueprints/BP_PlayerState.CurrentScore` (+ IncreaseAmount (`/Game/Blueprints/BP_PlayerState.CurrentScore` _asbp_player_state)) _asbp_player_state))

(fn `UserConstructionScript`)