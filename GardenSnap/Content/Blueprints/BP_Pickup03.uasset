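; BP_Pickup03 is a carrot score pickup that floats, spins and is collected when a player overlaps it.
; A self-restarting timeline started at BeginPlay moves and rotates the carrot mesh with relative offsets each update.
; On overlap, only the server casts the actor to BP_Player, adds ScoreToAdd through its BP_PlayerController, then destroys the pickup.
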(event `MovementAnim`
  (bind (_direction _nouvelle_piste_0) (`Timeline|Timeline` :!via `PlayFromStart`)
    (:`Update`
      (`SceneComponent.K2_AddRelativeLocation` (`self.carrot_carrot`) (* (`KismetMathLibrary.MakeVector` 0.0 0.0 _nouvelle_piste_0) (0.0 0.0 2.0)) false false)
      (`SceneComponent.K2_AddRelativeRotation` (`self.carrot_carrot`) (struct :`Yaw` 1.0) false false))
    (:`Finished`
      (`self.MovementAnim`))))

(event `self.ReceiveBeginPlay`
  (`self.MovementAnim`))

(event `self.ReceiveActorBeginOverlap`
  (params (OtherActor :type "Actor Object Reference"))
  (`/Engine/EditorBlueprintResources/ActorMacros.Switch Has Authority`
    (:`Authority`
      (bind _asbp_player (cast `/Game/Blueprints/BP_Player` OtherActor))
      (bind _asbp_player_controller (cast `/Game/Blueprints/BP_PlayerController` (`Pawn.GetController` _asbp_player)))
      (`/Game/Blueprints/BP_PlayerController.IncreaseScore` _asbp_player_controller (`self.ScoreToAdd`))
      (`self.K2_DestroyActor`))))

(fn `UserConstructionScript`)