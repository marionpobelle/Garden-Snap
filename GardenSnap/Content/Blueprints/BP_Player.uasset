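; Player character Blueprint that handles Enhanced Input movement and jumping, plus a meow sound on the P key.
; BeginPlay adds the InputMapPlayer mapping context, and IA_Move drives movement along the normalized camera right and forward vectors.
; P calls PlaySFXServer, which calls PlaySFXClient to print a debug string and play the 2D sound, a pairing named like a server-to-client RPC relay.
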(event `PlaySFXClient`
  (`KismetSystemLibrary.PrintString` "Pressed P")
  (`GameplayStatics.PlaySound2D` "/Game/Assets/Audio/Meow_Sound_Effect.Meow_Sound_Effect" 1.0 1.0 0.0 null null))

(event `PlaySFXServer`
  (`self.PlaySFXClient`))

(event `Key|P`
  (params (Key :type "Key Structure"))
  (:`Pressed`
    (`self.PlaySFXServer`)))

(event `self.ReceiveBeginPlay`
  (bind _asplayer_controller (cast `PlayerController` (`self.GetController`)))
  (`EnhancedInputSubsystemInterface.AddMappingContext` (pcsubsystem `EnhancedInputLocalPlayerSubsystem` _asplayer_controller) "/Game/Inputs/InputMapPlayer.InputMapPlayer" 0 (struct)))

(event `EnhancedInput|/Game/Inputs/IA_Jump`
  (params (ActionValue :type Boolean) (ElapsedSeconds :type "Float (double-precision)") (TriggeredSeconds :type "Float (double-precision)") (InputAction :type "InputAction Object Reference" :default "/Game/Inputs/IA_Jump.IA_Jump"))
  (:`Triggered`
    (`self.Jump`)))

(event `EnhancedInput|/Game/Inputs/IA_Move`
  (params (ActionValue :type "Vector2D Structure") (ElapsedSeconds :type "Float (double-precision)") (TriggeredSeconds :type "Float (double-precision)") (InputAction :type "InputAction Object Reference" :default "/Game/Inputs/IA_Move.IA_Move"))
  (bind _transformcomponent (`PlayerCameraManager.TransformComponent` (`GameplayStatics.GetPlayerCameraManager` 0)))
  (:`Triggered`
    (`self.AddMovementInput` (`KismetMathLibrary.Normal` (+ (* ActionValue_X (`SceneComponent.GetRightVector` _transformcomponent)) (* ActionValue_Y (`SceneComponent.GetForwardVector` _transformcomponent)))))))

(fn `UserConstructionScript`)